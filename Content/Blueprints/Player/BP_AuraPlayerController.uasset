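; Player controller that adds click-to-move to the controlled pawn, with a Niagara effect at the cursor hit point.
; When right-click is enabled and the cursor hits, it unpossesses the pawn, spawns its default AI controller and runs AI MoveTo.
; The camera stays on the cached pawn, which is repossessed when the move succeeds.
; Move input calls Possess only if that cached pawn reference is invalid.
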(event `self.ReceiveBeginPlay`
  (bind _output_get (set `self.ControlledPawn` (`self.K2_GetPawn`)))
  (`self.SetViewTargetWithBlend` _output_get))

(event `EnhancedInput|/Game/Blueprints/Input/Actions/IA_SetDestination_Click`
  (params (ActionValue :type Boolean) (ElapsedSeconds :type "Float (double-precision)") (TriggeredSeconds :type "Float (double-precision)") (InputAction :type "InputAction Object Reference" :default "/Game/Blueprints/Input/Actions/IA_SetDestination_Click.IA_SetDestination_Click"))
  (bind (_hitresult _returnvalue) (`self.GetHitResultUnderCursorByChannel` "TraceTypeQuery1"))
  (bind _controlledpawn (`self.ControlledPawn`))
  (bind (_bblockinghit _binitialoverlap _time _distance _location) (`GameplayStatics.BreakHitResult` _hitresult))
  (:`Triggered`
    (`NiagaraFunctionLibrary.SpawnSystemAtLocation` "/Game/Assets/Effects/Movement/NS_GroundSummonGreen.NS_GroundSummonGreen" _location)
    (if (and _returnvalue (`self.IsRightClickEnabled`))
      (`self.UnPossess`)
      (`Pawn.SpawnDefaultController` _controlledpawn)
      (`|AIMoveTo` _controlledpawn _location null
        (:`then`
          (`self.SetViewTargetWithBlend` (`self.ControlledPawn`)))
        (:`OnSuccess`
          (`self.Possess` (`self.ControlledPawn`)))))))

(event `EnhancedInput|/Game/Blueprints/Input/InputActions/IA_Move`
  (params (ActionValue :type "Vector2D Structure") (ElapsedSeconds :type "Float (double-precision)") (TriggeredSeconds :type "Float (double-precision)") (InputAction :type "InputAction Object Reference" :default "/Game/Blueprints/Input/InputActions/IA_Move.IA_Move"))
  (bind _controlledpawn (`self.ControlledPawn`))
  (:`Triggered`
    (`/Engine/EditorBlueprintResources/StandardMacros.IsValid` _controlledpawn
      (:`Is Not Valid`
        (`self.Possess` _controlledpawn)))))

(fn `UserConstructionScript`)